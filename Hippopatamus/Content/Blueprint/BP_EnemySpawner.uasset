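; BP_EnemySpawner is an actor that spawns BP_ENEMY1 enemies at its own location on a timed interval.
; BeginPlay sets a five-second rate, and a Delay on Tick paces the spawns until the spawn counter equals two.
; SpawnEnemy creates each enemy and prints its name and health as on-screen debug text.
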(event `self.ReceiveBeginPlay`
  (set `self.EnemySpawnRate` 5.0))

(event `self.ReceiveTick`
  (params (DeltaSeconds :type "Float (single-precision)"))
  (`KismetSystemLibrary.Delay` (`self.EnemySpawnRate`))
  (if (not (== (`self.SpawnCOunt`) 2.0))
    (`self.SpawnEnemy`)
    (bind _result (`/Engine/EditorBlueprintResources/StandardMacros.IncrementInt` (`self.SpawnCOunt`))
      (:`  `
        (set `self.SpawnCOunt` _result)
        (`KismetSystemLibrary.PrintString` "spawn enemy with " true true (struct :`G` 0.66 :`B` 1.0 :`A` 1.0) 20.0)))))

(fn `SpawnEnemy`
  (bind _returnvalue (`|SpawnActorFromClass` "/Game/Blueprint/BP_ENEMY1.BP_ENEMY1_C" (`KismetMathLibrary.MakeTransform` (`self.K2_GetActorLocation`)) "Undefined" "OverrideRootScale" null null))
  (`KismetSystemLibrary.PrintString` (`KismetStringLibrary.Concat_StrStr` "spawning enemy" (`KismetSystemLibrary.GetDisplayName` _returnvalue) "With Health: " (`KismetStringLibrary.Conv_DoubleToString` (`/Game/Blueprint/BP_ENEMY1.MyHealth` _returnvalue))) true true (struct :`G` 0.66 :`B` 1.0 :`A` 1.0) 20.0))

(fn `UserConstructionScript`)