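; Behavior tree task that sends an AI enemy toward the player location stored in the blackboard.
; If the enemy's pawn is not already at that point, it prints a debug message and issues an AI MoveTo.
; Both branches then wait a fixed delay before finishing as successful, without waiting on the move's result.
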(event `self.ReceiveExecute`
  (params (OwnerActor :type "Actor Object Reference"))
  (bind _returnvalue (`BTFunctionLibrary.GetBlackboardValueAsVector` (`self.myPlayerLocation`)))
  (bind _asbp_ai_enemy_controller (cast `/Game/Blueprint/enemy_AI_BP/BP_AI_ENEMY_CONTROLLER` OwnerActor))
  (bind _returnvalue_2 (`Controller.K2_GetPawn` _asbp_ai_enemy_controller))
  (if (not (== _returnvalue (`Actor.K2_GetActorLocation` _returnvalue_2) :`ErrorTolerance` 10.0))
    (`KismetSystemLibrary.PrintString` "moving")
    (`|AIMoveTo` _returnvalue_2 _returnvalue null 100.0
      (:`then`
        _)))
  (`KismetSystemLibrary.Delay` 10.0)
  (`self.FinishExecute` true))