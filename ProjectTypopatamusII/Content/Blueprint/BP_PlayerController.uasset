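; Player controller for a typing game where the player types through a random word stream shown on screen to charge an attack bar.
; On BeginPlay it creates the text widget, parses comma-separated words from a data table and builds the stream from random picks.
; Letter and Space key presses are compared, ignoring case, to the stream's first character.
; A match removes that character and refreshes the widget, and a correct Space also charges the player's attack bar.
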(event `self.ReceiveBeginPlay`
  (bind _returnvalue (`|CreateWidget` "/Game/Blueprint/WBP_PLAYER_TEXTS.WBP_PLAYER_TEXTS_C"))
  (bind _output_get (set `self.MyTextUI` _returnvalue))
  (`UserWidget.AddToViewport` _output_get 0)
  (`self.SetWordBankArray`)
  (`self.AssignPlayerWord`))

(event `self.ReceiveTick`
  (params (DeltaSeconds :type "Float (single-precision)")))

(event `Key|Y`
  (params (Key :type "Key Structure"))
  (:`Pressed`
    (`self.DetectKeyPress` Key)))

(event `Key|U`
  (params (Key :type "Key Structure"))
  (:`Pressed`
    (`self.DetectKeyPress` Key)))

(event `Key|Q`
  (params (Key :type "Key Structure"))
  (:`Pressed`
    (`self.DetectKeyPress` Key)))

(event `Key|M`
  (params (Key :type "Key Structure"))
  (:`Pressed`
    (`self.DetectKeyPress` Key)))

(event `Key|I`
  (params (Key :type "Key Structure"))
  (:`Pressed`
    (`self.DetectKeyPress` Key)))

(event `Key|E`
  (params (Key :type "Key Structure"))
  (:`Pressed`
    (`self.DetectKeyPress` Key)))

(event `Key|A`
  (params (Key :type "Key Structure"))
  (:`Pressed`
    (`self.DetectKeyPress` Key)))

(event `Key|Z`
  (params (Key :type "Key Structure"))
  (:`Pressed`
    (`self.DetectKeyPress` Key)))

(event `Key|V`
  (params (Key :type "Key Structure"))
  (:`Pressed`
    (`self.DetectKeyPress` Key)))

(event `Key|R`
  (params (Key :type "Key Structure"))
  (:`Pressed`
    (`self.DetectKeyPress` Key)))

(event `Key|N`
  (params (Key :type "Key Structure"))
  (:`Pressed`
    (`self.DetectKeyPress` Key)))

(event `Key|J`
  (params (Key :type "Key Structure"))
  (:`Pressed`
    (`self.DetectKeyPress` Key)))

(event `Key|F`
  (params (Key :type "Key Structure"))
  (:`Pressed`
    (`self.DetectKeyPress` Key)))

(event `Key|B`
  (params (Key :type "Key Structure"))
  (:`Pressed`
    (`self.DetectKeyPress` Key)))

(event `Key|W`
  (params (Key :type "Key Structure"))
  (:`Pressed`
    (`self.DetectKeyPress` Key)))

(event `Key|S`
  (params (Key :type "Key Structure"))
  (:`Pressed`
    (`self.DetectKeyPress` Key)))

(event `Key|O`
  (params (Key :type "Key Structure"))
  (:`Pressed`
    (`self.DetectKeyPress` Key)))

(event `Key|K`
  (params (Key :type "Key Structure"))
  (:`Pressed`
    (`self.DetectKeyPress` Key)))

(event `Key|G`
  (params (Key :type "Key Structure"))
  (:`Pressed`
    (`self.DetectKeyPress` Key)))

(event `Key|C`
  (params (Key :type "Key Structure"))
  (:`Pressed`
    (`self.DetectKeyPress` Key)))

(event `Key|X`
  (params (Key :type "Key Structure"))
  (:`Pressed`
    (`self.DetectKeyPress` Key)))

(event `Key|T`
  (params (Key :type "Key Structure"))
  (:`Pressed`
    (`self.DetectKeyPress` Key)))

(event `Key|P`
  (params (Key :type "Key Structure"))
  (:`Pressed`
    (`self.DetectKeyPress` Key)))

(event `Key|L`
  (params (Key :type "Key Structure"))
  (:`Pressed`
    (`self.DetectKeyPress` Key)))

(event `Key|H`
  (params (Key :type "Key Structure"))
  (:`Pressed`
    (`self.DetectKeyPress` Key)))

(event `Key|D`
  (params (Key :type "Key Structure"))
  (:`Pressed`
    (`self.DetectKeyPress` Key)))

(event `Key|SpaceBar`
  (params (Key :type "Key Structure"))
  (:`Pressed`
    (`self.DetectKeyPress` Key)))

(fn `AssignPlayerWord`
  (bind _returnvalue (`KismetStringLibrary.Trim` (`KismetStringLibrary.JoinStringArray` (`self.CurrentWordStream`))))
  (for _ (range 501)
    (`KismetArrayLibrary.Array_Add` (`self.CurrentWordStream`) (`KismetArrayLibrary.Array_Random` (`self.properWords`))))
  (`KismetSystemLibrary.PrintString` _returnvalue)
  (bind _output_get (set `self.CurrentWordStream` (`KismetStringLibrary.ParseIntoArray` _returnvalue)))
  (`/Game/Blueprint/WBP_PLAYER_TEXTS.UpdateText` (`self.MyTextUI`) _output_get))

(fn `DetectKeyPress`
  (params (Key :type "Key Structure" :default "None"))
  (`self.ProcessCharacter` (`KismetTextLibrary.Conv_TextToString` (`KismetInputLibrary.Key_GetDisplayName` Key))))

(fn `ProcessCharacter`
  (params (Character :type String))
  (if (`KismetStringLibrary.EqualEqual_StrStr` Character "Space Bar")
    (if (`KismetStringLibrary.EqualEqual_StrStr` (`KismetStringLibrary.ToUpper` (`KismetStringLibrary.GetSubstring` (`KismetStringLibrary.JoinStringArray` (`self.CurrentWordStream`)))) (`self.Space`))
      (`/Game/Blueprint/BP_Player.ChargeAttackBar` (`self.MyPlayerRef`))
      (set `self.CurrentWordStream` (`KismetStringLibrary.ParseIntoArray` (`KismetStringLibrary.RightChop` (`KismetStringLibrary.JoinStringArray` (`self.CurrentWordStream`)) 1) " " false) :!label _label)
      (`/Game/Blueprint/WBP_PLAYER_TEXTS.UpdateText` (`self.MyTextUI`) (`self.CurrentWordStream`)))
    (elif (`KismetStringLibrary.EqualEqual_StrStr` (`KismetStringLibrary.ToUpper` (`KismetStringLibrary.GetSubstring` (`KismetStringLibrary.JoinStringArray` (`self.CurrentWordStream`)))) Character)
      (goto _label))))

(fn `SetWordBankArray`
  (bind _output_get (set `self.DataTableWords` "/Game/Texts/WordBank_-_Sheet1.WordBank_-_Sheet1"))
  (bind _outrownames (`DataTableFunctionLibrary.GetDataTableRowNames` _output_get))
  (for _array_element _outrownames
    (bind _returnvalue (`|GetDataTableRow` (`self.DataTableWords`) _array_element)
      (:`then`
        (`KismetArrayLibrary.Array_Add` (`self.wordsArray`) (`.Words_2_B3B3357B22DD44318B8C8C800A134A8D` (break `/Game/Texts/columnStruct` _returnvalue))))))
  (set `self.properWords` (`KismetStringLibrary.ParseIntoArray` (`KismetStringLibrary.JoinStringArray` (`self.wordsArray`)) ",")))

(fn `UserConstructionScript`)