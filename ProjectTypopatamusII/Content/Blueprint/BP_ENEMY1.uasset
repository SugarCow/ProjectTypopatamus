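; BP_ENEMY1 is an enemy with a health-bar widget that holds its health.
; BeginPlay initialises health and attack power, registers the enemy on BP_Player, and spawns an AI controller to possess it.
; Tick destroys the enemy when widget health reaches zero.
; Attack subtracts damage from a target's health, but the overlap event is empty, its attack loop is disconnected, and CreateHealthBarWidget is never called here.
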(event `self.ReceiveBeginPlay`
  (bind _aswbp_enemy_health (cast `/Game/Blueprint/WBP_ENEMY_HEALTH` (`WidgetComponent.GetUserWidgetObject` (`self.Health Widget`))))
  (bind _output_get (set `self.MyHealthBar` _aswbp_enemy_health))
  (set `/Game/Blueprint/WBP_ENEMY_HEALTH.Health ` 100.0 _output_get)
  (set `self.MyAttack ` 10.0)
  (bind _asbp_player (cast `/Game/Blueprint/BP_Player` (`GameplayStatics.GetPlayerPawn` 0)))
  (set `self.MyPlayer` _asbp_player)
  (bind _returnvalue (`|SpawnActorFromClass` "/Game/Blueprint/enemy_AI_BP/BP_AI_ENEMY_CONTROLLER.BP_AI_ENEMY_CONTROLLER_C" (`KismetMathLibrary.MakeTransform` (`self.K2_GetActorLocation`)) "Undefined" "OverrideRootScale" null null))
  (`Controller.Possess` _returnvalue self)
  (set `/Game/Blueprint/BP_Player.MyEmemy` self (`self.MyPlayer`)))

(event `self.ReceiveTick`
  (params (DeltaSeconds :type "Float (single-precision)"))
  (if (<= (`/Game/Blueprint/WBP_ENEMY_HEALTH.Health ` (`self.MyHealthBar`)) 0.0)
    (`self.K2_DestroyActor`)))

(event `self.AttackModeCollision.OnComponentBeginOverlap`
  (params (OverlappedComponent :type "PrimitiveComponent Object Reference") (OtherActor :type "Actor Object Reference") (OtherComp :type "PrimitiveComponent Object Reference") (OtherBodyIndex :type Integer) (bFromSweep :type Boolean) (SweepResult :type "HitResult Structure (by ref)")))

(fn `Attack`
  (params (Target :type "/Game/Blueprint/BP_Player Object Reference"))
  (set `/Game/Blueprint/BP_Player.Health ` (- (`/Game/Blueprint/BP_Player.Health ` Target) (`self.MyAttack `)) Target))

(fn `CreateHealthBarWidget`
  (bind _returnvalue (`|CreateWidget` "/Game/Blueprint/WBP_ENEMY_HEALTH.WBP_ENEMY_HEALTH_C"))
  (bind _output_get (set `self.MyHealthBar` _returnvalue))
  (set `/Game/Blueprint/WBP_ENEMY_HEALTH.BP ENEMY1 ref` self _output_get))

(fn `UserConstructionScript`)